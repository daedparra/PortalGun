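; FPSPlayerController is a first-person player controller that turns player input into actions on the possessed FPSCharacter.
; On BeginPlay it casts the controlled pawn to FPSCharacter and caches it.
; Tick applies forward and right movement along the actor's axes, while look axes feed pitch and yaw.
; Action inputs forward to the character for jumping, primary and secondary fire, four weapon slots, crouching and sprinting.
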(event EventTick
  (params (DeltaSeconds :type Float%20%28single-precision%29))
  (CallFunction|ApplyMoveInput))

(event EventBeginPlay
  (CallFunction|Initialize))

(event Input|ActionEvents|InputActionJump
  (params (Key :type Key%20Structure))
  (bind _fpscharacter (Variables|Default|GetFPSCharacter))
  (:Pressed
    (Character|Jump _fpscharacter))
  (:Released
    (Character|StopJumping _fpscharacter)))

(event Input|ActionEvents|InputActionShoot
  (params (Key :type Key%20Structure))
  (bind _fpscharacter (Variables|Default|GetFPSCharacter))
  (:Pressed
    (Default|StartFire _fpscharacter false))
  (:Released
    (Default|StopFire _fpscharacter)))

(event Input|ActionEvents|InputActionWeapon0
  (params (Key :type Key%20Structure))
  (:Pressed
    (Default|SwaptoWeapon (Variables|Default|GetFPSCharacter))))

(event Input|ActionEvents|InputActionWeapon1
  (params (Key :type Key%20Structure))
  (:Pressed
    (Default|SwaptoWeapon (Variables|Default|GetFPSCharacter) 1)))

(event Input|ActionEvents|InputActionWeapon2
  (params (Key :type Key%20Structure))
  (:Pressed
    (Default|SwaptoWeapon (Variables|Default|GetFPSCharacter) 2)))

(event Input|ActionEvents|InputActionWeapon3
  (params (Key :type Key%20Structure))
  (:Pressed
    (Default|SwaptoWeapon (Variables|Default|GetFPSCharacter) 3)))

(event Input|ActionEvents|InputActionFire2
  (params (Key :type Key%20Structure))
  (bind _fpscharacter (Variables|Default|GetFPSCharacter))
  (:Pressed
    (Default|StartFire _fpscharacter true))
  (:Released
    (Default|StopFire _fpscharacter)))

(event Input|ActionEvents|InputActionCrouch
  (params (Key :type Key%20Structure))
  (bind _fpscharacter (Variables|Default|GetFPSCharacter))
  (:Pressed
    (Default|StartCrouch _fpscharacter))
  (:Released
    (Default|StopCrouch _fpscharacter)))

(event Input|ActionEvents|InputActionSprint
  (params (Key :type Key%20Structure))
  (bind _fpscharacter (Variables|Default|GetFPSCharacter))
  (:Pressed
    (Default|StartSprint _fpscharacter))
  (:Released
    (Default|StopSprint _fpscharacter)))

(event Input|AxisEvents|InputAxisLookUp
  (params (AxisValue :type Float%20%28single-precision%29))
  (CallFunction|ApplyLookInput true AxisValue))

(event Input|AxisEvents|InputAxisLookRight
  (params (AxisValue :type Float%20%28single-precision%29))
  (CallFunction|ApplyLookInput false AxisValue))

(fn ConstructionScript)

(fn ApplyMoveInput
  (bind _fpscharacter (Variables|Default|GetFPSCharacter))
  (bind _fpscharacter_2 (Variables|Default|GetFPSCharacter))
  (Pawn|Input|AddMovementInput _fpscharacter_2 (Transformation|GetActorForwardVector _fpscharacter_2) (Input|AxisValues|GetMoveForward) false)
  (Pawn|Input|AddMovementInput _fpscharacter (Transformation|GetActorRightVector _fpscharacter) (Input|AxisValues|GetMoveRight) false))

(fn Initialize
  (bind _asfpscharacter (Utilities|Casting|CastToFPSCharacter (Pawn|GetControlledPawn)))
  (Variables|Default|SetFPSCharacter _asfpscharacter))

(fn ApplyLookInput
  (params (LookUp :type Boolean) (AxisValue :type Float%20%28single-precision%29))
  (bind _fpscharacter (Variables|Default|GetFPSCharacter))
  (if LookUp
    (Pawn|Input|AddControllerPitchInput _fpscharacter AxisValue)
    (else
      (Pawn|Input|AddControllerYawInput _fpscharacter AxisValue))))