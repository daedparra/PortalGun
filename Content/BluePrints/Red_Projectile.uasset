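; Red portal projectile that places a red portal on the surface it is about to hit, replacing the existing one.
; Each Tick it line traces a short distance forward on the Visibility channel.
; A hit destroys the first existing RedHors and RedPortal, then the projectile itself.
; An upward-facing impact normal spawns RedHors and any other spawns RedPortal, nudged off the impact point along the normal.
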(event EventTick
  (params (DeltaSeconds :type Float%20%28single-precision%29))
  (bind _defaultsceneroot (Variables|Default|GetDefaultSceneRoot))
  (bind _returnvalue (Transformation|GetWorldTransform _defaultsceneroot))
  (bind _location (Math|Transform|BreakTransform _returnvalue))
  (bind (_outhit _returnvalue_2) (Collision|LineTraceByChannel _location (+ _location (* (Math|Vector|GetForwardVector _defaultsceneroot) 1e+02)) "TraceTypeQuery1" false 0 "None"))
  ;[1 1 1] If it collide with the wall first all other portals will be deleted to spawn a new portal
  (if _returnvalue_2
    (bind _outactors (Actor|GetAllActorsOfClass "/Game/BluePrints/RedHors.RedHors_C"))
    (Actor|DestroyActor (Utilities|Array|Get(acopy) _outactors))
    (bind _outactors_2 (Actor|GetAllActorsOfClass "/Game/BluePrints/RedPortal.RedPortal_C"))
    (Actor|DestroyActor (Utilities|Array|Get(acopy) _outactors_2))
    (if (!= (.HitActor (Collision|BreakHitResult _outhit)) self)
      (Actor|DestroyActor)
      ;[1 1 1] depending on what it hit, a different portal will be spawn
      (if (== (.Z (Math|Vector|BreakVector (.ImpactNormal (Collision|BreakHitResult _outhit)))) 1.0)
        (Game|SpawnActorfromClass "/Game/BluePrints/RedHors.RedHors_C" (Math|Conversions|ToTransform(Vector) (+ (.ImpactPoint (Collision|BreakHitResult _outhit)) (.ImpactNormal (Collision|BreakHitResult _outhit)))) "AlwaysSpawn" 0 0)
        (else
          (Game|SpawnActorfromClass "/Game/BluePrints/RedPortal.RedPortal_C" (Math|Conversions|ToTransform(Vector) (+ (.ImpactPoint (Collision|BreakHitResult _outhit)) (.ImpactNormal (Collision|BreakHitResult _outhit)))) "AlwaysSpawn" 0 0))))))

(fn ConstructionScript)