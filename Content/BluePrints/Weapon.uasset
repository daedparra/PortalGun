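; Weapon Blueprint that handles automatic fire, spawning bullets with muzzle flash and sound while the trigger is held.
; Stats load from a data table row on BeginPlay; Tick decays spread and fires whenever the RPM cooldown allows.
; Each shot line-traces from the look transform for an aim point, then rotates the bullet from the muzzle toward it with random spread.
; Spread is clamped 0–1, grows per shot and scales the data-driven spread angle.
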(event Custom|StartFire
  (params (WeaponfireInfo :type Weapon%20Fire%20Info%20Structure))
  (Variables|Default|SetWeaoinfireinfo WeaponfireInfo)
  (Variables|Default|SetWantsTofire true))

(event Custom|StopFire
  (Variables|Default|SetWantsTofire false))

(event EventBeginPlay
  (CallFunction|LoadData))

(event EventTick
  (params (DeltaSeconds :type Float%20%28single-precision%29))
  (bind _weaoinfireinfo (Variables|Default|GetWeaoinfireinfo))
  (bind (_lookdirection _muzzledirection _instigatior _weaponmesh _bulletclass) (Utilities|Struct|BreakWeaponFireInfo _weaoinfireinfo))
  (CallFunction|DecaySpread DeltaSeconds)
  (Utilities|AttempetFire
    (:Success
      (Variables|Default|SetBulletClass _bulletclass)
      (CallFunction|Shoot (Transformation|GetWorldTransform _muzzledirection) (Transformation|GetWorldTransform _lookdirection) _instigatior _weaponmesh))))

(fn Shoot
  (params (Transform :type Transform) (Lookdirection :type Transform) (Instigator :type Pawn%20Object%20Reference) (WeaponMesh :type Skeletal%20Mesh%20Component%20Object%20Reference))
  (bind _location (Math|Transform|BreakTransform Transform))
  (bind _aimdirection (CallFunction|GetAimDirection Lookdirection))
  (Game|SpawnActorfromClass (Variables|Default|GetBulletClass) (Math|Transform|MakeTransform _location (CallFunction|AddInaccuracy (Math|Rotator|FindLookatRotation _location _aimdirection))) "AlwaysSpawn" 0 Instigator)
  (Effects|SpawnEmitterAttached (Variables|Default|GetMuzzleFlair) WeaponMesh "BarrelAttachmentPoint" "0, 0, 0" "0, 0, 0" "1.000000,1.000000,1.000000" "SnapToTarget")
  (Audio|SpawnSoundAttached "/Game/Audio/WeaponFire.WeaponFire" WeaponMesh "BarrelAttachmentPoint" "0, 0, 0" "0, 0, 0" "SnapToTarget")
  (CallFunction|ModifySpread (.SpreadFireIncrement (Utilities|Struct|BreakWeaponData (Variables|Default|GetData))))
  (Default|CallWeaponFre))

(fn GetAimDirection
  (params (Lookdirection :type Transform))
  (bind (_location _rotation) (Math|Transform|BreakTransform Lookdirection))
  (bind _returnvalue (Math|Vector|GetForwardVector _rotation))
  (bind _returnvalue_2 (* _returnvalue 1e+04))
  (bind _returnvalue_3 (+ _returnvalue_2 _location))
  (bind (_outhit _returnvalue_4) (Collision|LineTraceByChannel _location _returnvalue_3 "TraceTypeQuery1" true 0 "ForDuration" true "(R=1.000000,G=0.000000,B=0.000000,A=1.000000)" "(R=0.000000,G=1.000000,B=0.000000,A=1.000000)" 1.0))
  (if _returnvalue_4
    ;[1 1 1] Aim location (hit something)
    (return (.ImpactPoint (Collision|BreakHitResult _outhit)))
    (else
      ;[1 1 1] Direction from muzzle to infiitely far off point
      (return _returnvalue_3))))

(fn LoadData
  (bind _datatablename (Variables|Default|GetDataTableName))
  (bind _returnvalue (Utilities|GetDataTableRow "/Game/Data/WeaponDataTable.WeaponDataTable" _datatablename)
    (:then
      (Variables|Default|SetData _returnvalue))
    (:RowNotFound
      (Development|PrintString (Utilities|String|Append "coud not find weapon data with name " (Utilities|String|ToString(Name) _datatablename)) true true "(R=1.000000,G=0.000000,B=0.028928,A=1.000000)"))))

(fn CanFire
  (return (>= (Utilities|Time|GetGameTimeinSeconds) (+ (Variables|Default|GetLastFiretime) (/ 6e+01 (.RPM (Utilities|Struct|BreakWeaponData (Variables|Default|GetData))))))))

(fn AddInaccuracy
  (params (Rotator :type Rotator))
  (bind _data (Variables|Default|GetData))
  (bind _spread (Variables|Default|GetSpread))
  (bind _spreadangle (Utilities|Struct|BreakWeaponData _data))
  (return (Math|Rotator|CombineRotators Rotator (Math|Rotator|MakeRotator (* (Math|Random|RandomFloatinRange -1.0 1.0) (Variables|Default|GetSpread) _spreadangle) (* (Math|Random|RandomFloatinRange -1.0 1.0) _spreadangle _spread) (* _spread _spreadangle (Math|Random|RandomFloatinRange -1.0 1.0))))))

(fn ModifySpread
  (params (Amount :type Float%20%28single-precision%29))
  (Variables|Default|SetSpread (Math|Float|Clamp(Float) (+ Amount (Variables|Default|GetSpread)) 0.0)))

(fn DecaySpread
  (params (DeltaTime :type Float%20%28single-precision%29))
  (CallFunction|ModifySpread (* DeltaTime (.SpreadDecay (Utilities|Struct|BreakWeaponData (Variables|Default|GetData))) -1.0)))