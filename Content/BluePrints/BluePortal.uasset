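; Blue portal actor that teleports the player to a red portal when the player overlaps it.
; It takes the first RedPortal found in the level and moves the pawn to that location, keeping its rotation.
; An IsTeleporting flag set on the destination guards against bouncing back: an overlap while this portal's flag is set only clears it after a short delay.
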(event Collision|EventActorBeginOverlap
  (params (OtherActor :type Actor%20Object%20Reference))
  (bind _returnvalue (Game|Player|GetPlayerPawn 0))
  (if (not (!= OtherActor (Game|GetPlayerCharacter 0)))
    (if (Variables|Default|GetisTeleporting)
      ;[1 1 1] If he arrives from the other portal, it will do nothing
      (Utilities|FlowControl|Delay 0.5)
      (Variables|Default|SetisTeleporting false)
      (else
        ;[1 1 1] It will search for the other portal, to search for it. And then take the pawn to the other character
        (bind _outactors (Actor|GetAllActorsOfClass "/Game/BluePrints/RedPortal.RedPortal_C"))
        (Variables|/Game/BluePrints/RedPortal.RedPortal_C|SetisTeleporting (Utilities|Array|Get(acopy) _outactors) true)
        (Transformation|Teleport _returnvalue (Transformation|GetActorLocation (Utilities|Array|Get(acopy) _outactors)) (Transformation|GetActorRotation _returnvalue))))))

(fn ConstructionScript)