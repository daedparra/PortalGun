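; Bullet projectile actor that damages the first other actor it hits, then destroys itself.
; Each tick it line-traces forward from its root along the Visibility channel by TraceDistance, and it also listens for overlaps.
; Both paths call ActorHit, which ignores itself, prints the hit actor's name, applies Damage credited to the instigator's controller, and destroys the bullet.
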(event EventTick
  (params (DeltaSeconds :type Float%20%28single-precision%29))
  (bind _defaultsceneroot (Variables|Default|GetDefaultSceneRoot))
  (bind _returnvalue (Transformation|GetWorldTransform _defaultsceneroot))
  (bind _location (Math|Transform|BreakTransform _returnvalue))
  (bind (_outhit _returnvalue_2) (Collision|LineTraceByChannel _location (+ _location (* (Math|Vector|GetForwardVector _defaultsceneroot) (Variables|Default|GetTraceDistance))) "TraceTypeQuery1" false 0 "None"))
  (if _returnvalue_2
    (CallFunction|ActorHit (.HitActor (Collision|BreakHitResult _outhit)))))

(event Collision|EventActorBeginOverlap
  (params (OtherActor :type Actor%20Object%20Reference))
  (CallFunction|ActorHit OtherActor))

(fn ConstructionScript)

(fn ActorHit
  (params (Actor :type Actor%20Object%20Reference))
  (if (!= Actor self)
    (Development|PrintString (Utilities|String|Append (Utilities|GetObjectName Actor) "") true true "(R=1.000000,G=0.949772,B=0.000000,A=1.000000)")
    (Game|Damage|ApplyDamage Actor (Variables|Default|GetDamage) (Pawn|GetController (Variables|Actor|GetInstigator)) self)
    (Actor|DestroyActor)))