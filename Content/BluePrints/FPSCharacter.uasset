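; First-person player character Blueprint with sprint, crouch, a crosshair HUD and four weapons including a portal gun.
; Swapping weapons stops all firing, attaches the mesh and muzzle to sockets, and shows only that mesh.
; Firing delegates to the equipped weapon, with the portal gun, detected by mesh name, choosing red or blue projectiles by mouse button.
; Each tick selects movement values, sprinting only on forward input, then sets speed and lerps capsule height, FOV and vignette.
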(event Custom|StopSprint
  (Variables|Default|SetWantstosprint false))

(event Custom|StartSprint
  (Variables|Default|SetWantstosprint true))

(event Custom|StartCrouch
  (Variables|Default|SetWantstocrouch true))

(event Custom|StopCrouch
  (Variables|Default|SetWantstocrouch false))

(event EventBeginPlay
  (CallFunction|InitializeHud)
  (Variables|Default|SetWeapons (Utilities|Array|MakeArray (Variables|Default|GetPistol) (Variables|Default|GetSMG) (Variables|Default|GetShotGun) (Variables|Default|GetPortalGun)))
  (Variables|Default|SetWeaponMeshes (Utilities|Array|MakeArray (Variables|Default|GetPistolMesh) (Variables|Default|GetSMGMesh) (Variables|Default|GetShotGunMesh) (Variables|Default|GetPortalGunMesh)))
  (CallFunction|SwaptoWeapon))

(event EventTick
  (params (DeltaSeconds :type Float%20%28single-precision%29))
  (CallFunction|Resolvemovemntvalues)
  (CallFunction|ApplyMovementValues))

(fn ConstructionScript)

(fn StartFire
  (params (isRight :type Boolean))
  (bind _self self)
  (bind _muzzle (Variables|Default|GetMuzzle))
  (bind _equipedweaponmesh (Variables|Default|GetEquipedWeaponMesh))
  (bind _lookdirection (Variables|Default|GetLookDirection))
  ;[1 1 1] if the user is or not on the portal gun
  (if (Utilities|Enum|NotEqual(Enum) (Utilities|GetObjectName _equipedweaponmesh) "PortalGunMesh")
    (bind _output_get (Variables|Default|SetBulletClass "/Game/BluePrints/Bullet.Bullet_C"))
    (Default|StartFire (Variables|Default|GetEquippedWeapon) (Utilities|Struct|MakeWeaponFireInfo _lookdirection _muzzle _self _equipedweaponmesh _output_get))
    (else
      ;[1 1 1] Right or Left Click
      (if isRight
        (bind _output_get_2 (Variables|Default|SetBulletClass "/Game/BluePrints/Red_Projectile.Red_Projectile_C"))
        (Default|StartFire (Variables|Default|GetEquippedWeapon) (Utilities|Struct|MakeWeaponFireInfo _lookdirection _muzzle _self _equipedweaponmesh _output_get_2))
        (else
          (bind _output_get_3 (Variables|Default|SetBulletClass "/Game/BluePrints/Blure_Projectile.Blure_Projectile_C"))
          (Default|StartFire (Variables|Default|GetEquippedWeapon) (Utilities|Struct|MakeWeaponFireInfo _lookdirection _muzzle _self _equipedweaponmesh _output_get_3)))))))

(fn AttachART
  (params (WeaponMesh :type Skeletal%20Mesh%20Component%20Object%20Reference))
  (bind _mesh (Variables|Character|GetMesh))
  ;[1 1 1] armMesh
  (Transformation|AttachComponentToComponent _mesh (Variables|Default|GetCamera) "None" "KeepWorld" "KeepWorld" "KeepWorld" true)
  ;[1 1 1] WeaponMesh
  (Transformation|AttachComponentToComponent WeaponMesh _mesh "WeaponSocket" "SnapToTarget" "SnapToTarget" "SnapToTarget" true)
  ;[1 1 1] attaches the muzzle
  (Transformation|AttachComponentToComponent (Variables|Default|GetMuzzle) WeaponMesh "BarrelAttachmentPoint" "SnapToTarget" "SnapToTarget" "SnapToTarget" true))

(fn InitializeHud
  (bind _returnvalue (UserInterface|CreateWidget "/Game/BluePrints/Crosshair.Crosshair_C"))
  (UserInterface|Viewport|AddtoViewport _returnvalue 0))

(fn SwaptoWeapon
  (params (WeaponIndex :type Integer))
  (bind _weaponmeshes (Variables|Default|GetWeaponMeshes))
  (bind _output (Utilities|Array|Get(acopy) _weaponmeshes WeaponIndex))
  (CallFunction|StopFiringAll)
  (Variables|Default|SetEquippedWeapon (Utilities|Array|Get(acopy) (Variables|Default|GetWeapons) WeaponIndex))
  (CallFunction|AttachART _output)
  (Variables|Default|SetEquipedWeaponMesh _output)
  (CallFunction|ToggleWeaponArt WeaponIndex))

(fn ToggleWeaponArt
  (params (MeshIndex :type Integer))
  (bind _weaponmeshes (Variables|Default|GetWeaponMeshes))
  (for _array_element _weaponmeshes
    (Rendering|SetVisibility _array_element false false))
  (Rendering|SetVisibility (Utilities|Array|Get(acopy) _weaponmeshes MeshIndex) true false))

(fn StopFire
  (Default|StopFire (Variables|Default|GetEquippedWeapon)))

(fn StopFiringAll
  (for _array_element (Variables|Default|GetWeapons)
    (Default|StopFire _array_element)))

(fn ApplyMovementValues
  (bind _currentmovementvalues (Variables|Default|GetCurrentMovementValues))
  (bind (_movespeed _halfheight _accracymodifier _fov _vignette) (Utilities|Struct|BreakMovemetnValues _currentmovementvalues))
  (Variables|/Script/Engine.CharacterMovementComponent|SetMaxWalkSpeed (Variables|Character|GetCharacterMovement) _movespeed)
  (CallFunction|LerpHalfHeight _halfheight)
  (CallFunction|LerpFOV _fov)
  (CallFunction|LerpViniet _vignette))

(fn Resolvemovemntvalues
  (if (and (Variables|Default|GetWantstosprint) (>= (.X (Math|Vector|BreakVector (Math|Transform|InverseTransformDirection (Transformation|GetWorldTransform (Variables|Collision|GetCapsuleComponent)) (Pawn|Components|PawnMovement|GetLastInputVector (Variables|Character|GetCharacterMovement))))) 0.5))
    (Variables|Default|SetCurrentMovementValues (Variables|Default|GetSprintMoveValues))
    (elif (Variables|Default|GetWantstocrouch)
      (Variables|Default|SetCurrentMovementValues (Variables|Default|GetCrouchMovementValues))
      (else
        (Variables|Default|SetCurrentMovementValues (Variables|Default|GetRunMoveMentsValues))))))

(fn LerpHalfHeight
  (params (HalfHeight :type Float%20%28single-precision%29))
  (Components|Capsule|SetCapsuleHalfHeight (Variables|Collision|GetCapsuleComponent) (Math|Float|Lerp (Variables|/Script/Engine.CapsuleComponent|GetCapsuleHalfHeight (Variables|Collision|GetCapsuleComponent)) HalfHeight (* (Utilities|Time|GetWorldDeltaSeconds) 1e+01)) true))

(fn LerpFOV
  (params (targetFOV :type Float%20%28single-precision%29))
  (Camera|SetFieldOfView (Variables|Default|GetCamera) (Math|Float|Lerp (Variables|/Script/Engine.CameraComponent|GetFieldOfView (Variables|Default|GetCamera)) targetFOV (* (Utilities|Time|GetWorldDeltaSeconds) 1e+01))))

(fn LerpViniet
  (params (TargetVigniete :type Float%20%28single-precision%29))
  (Variables|/Script/Engine.CameraComponent|SetPostProcessSettings (Variables|Default|GetCamera) (Utilities|Struct|MakePostProcessSettings (Math|Float|Lerp (Utilities|Struct|BreakPostProcessSettings (Variables|/Script/Engine.CameraComponent|GetPostProcessSettings (Variables|Default|GetCamera))) TargetVigniete (* (Utilities|Time|GetWorldDeltaSeconds) 1e+01)))))